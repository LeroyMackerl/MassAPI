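; BP_MassAPINodeDisplay is a showcase Blueprint for MassAPI nodes, with no connected gameplay logic.
; It groups smart nodes for flags, fragments and tags on entity handles or template data, alongside entity query, build and destroy nodes.
; Usage notes cover deferred operation, type-filtered pins and per-member fragment setting.
; A deprecated section lays out the older separate entity and template nodes, including shared and const shared fragment variants.
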(fn `UserConstructionScript`)