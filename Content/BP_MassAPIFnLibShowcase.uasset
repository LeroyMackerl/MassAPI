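; Showcase Blueprint for the MassAPI function library, laying out its Mass entity nodes as unconnected, never-executed examples with usage notes.
; Smart nodes edit fragments, tags and named flags on entity handles or template data, with optional deferral and per-member fragment writes.
; Other examples build entities from templates, query, iterate and destroy them.
; A deprecated section retains the older entity-specific and template-specific nodes, including shared fragment operations.
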(event `CustomEvent`
  (params (EntityHandle :type "EntityHandle Structure"))
  ; How To Use
  ;; 2. Check the Deferred checkbox if you want deferred operation
)

(fn `UserConstructionScript`)